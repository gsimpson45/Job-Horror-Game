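; BP_MenuMusic is a sound manager actor that plays the menu music as a 2D sound, starting it with a fade-in on BeginPlay.
; StartSound spawns the track, keeps the audio component in CurrMenuMusic and optionally fades it in.
; EndSound prints a debug message and fades out the stored component only when Fade is true and it is valid; without Fade the music keeps playing.
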(event `self.ReceiveBeginPlay`
  (`self.startSound` true))

(event `/Game/Sounds/BP_SoundManagers/SoundCalls.startSound`
  (params (fade :type Boolean))
  (if fade
    (bind _returnvalue (`GameplayStatics.SpawnSound2D` "/Game/Sounds/Music/MenuMusic.MenuMusic" 1.0 1.0 0.0 null))
    (set `self.currMenuMusic` _returnvalue)
    (`AudioComponent.FadeIn` (`self.currMenuMusic`) 2.0 1.0 0.0 "Linear")
    (else
      (bind _returnvalue_2 (`GameplayStatics.SpawnSound2D` "/Game/Sounds/Music/MenuMusic.MenuMusic" 1.0 1.0 0.0 null))
      (set `self.currMenuMusic` _returnvalue_2))))

(event `/Game/Sounds/BP_SoundManagers/SoundCalls.endSound`
  (params (fade :type Boolean))
  (`KismetSystemLibrary.PrintString` "ending sound")
  (if fade
    (bind _currmenumusic (`self.currMenuMusic`)
      (:`then`
        (`AudioComponent.FadeOut` _currmenumusic 1.0 0.0 "Linear"))
      (:`else`))))

(fn `UserConstructionScript`)