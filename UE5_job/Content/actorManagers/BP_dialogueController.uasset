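; BP_dialogueController is an actor that starts and ends dialogue from a supplied DataTable.
; StartDialogue creates a Dialogue widget, then either adds it to the viewport or sends it to the first Screen actor's in-world PC widget.
; Once talking is done, Tick restores game-only input unless the player sits in the pcChair-tagged chair.
; EndDialogue removes the finished widget and notifies the calling actor.
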(event `self.ReceiveBeginPlay`)

(event `/Game/actorManagers/startTalking.startDialogue`
  (params (dialogueTable :type "DataTable Object Reference") (`sendToPC?` :type Boolean) (CallingActor :type "Actor Object Reference"))
  (set `self.Calling Actor` CallingActor)
  (set `self.Send to PC?` `sendToPC?`)
  (bind _returnvalue (`|CreateWidget` "/Game/widgets/dialogueWidget/dialogue.dialogue_C" (`GameplayStatics.GetPlayerController` 0)))
  (bind _output_get (set `self.widget` _returnvalue))
  (bind _asdialogue (cast `/Game/widgets/dialogueWidget/dialogue` _output_get))
  (set `/Game/widgets/dialogueWidget/dialogue.dialogueDataTable` dialogueTable _asdialogue)
  (set `/Game/widgets/dialogueWidget/dialogue.startRowIndex` 0 _asdialogue)
  (if (`self.Send to PC?`)
    (bind _outactors (`GameplayStatics.GetAllActorsOfClass` "/Game/screen.screen_C"))
    (bind _asscreen (cast `/Game/screen` (`|GetArrayItem` _outactors)))
    (message `/Game/actorManagers/ComputerDialogue.startDialogueOnPC` (`WidgetComponent.GetWidget` (`/Game/screen.Widget` _asscreen)) (`self.widget`))
    (`KismetSystemLibrary.PrintString` "Sending dialogue to pc")
    (else
      (`UserWidget.AddToViewport` (`self.widget`) 0))))

(event `/Game/actorManagers/ComputerDialogue.startDialogueOnPC`
  (params (dialogue :type "Widget Object Reference")))

(event `self.ReceiveTick`
  (params (DeltaSeconds :type "Float (single-precision)"))
  (bind _widget (`self.widget`)
    (:`then`
      (if (`/Game/widgets/dialogueWidget/dialogue.doneTalking?` _widget)
        (bind _outactors (`GameplayStatics.GetAllActorsOfClassWithTag` "/Game/InteractableActors/BP_Chair.BP_Chair_C" "pcChair"))
        (bind _isplayersitting (message `/Game/widgets/objectInteraction/BPI_PlayerSit.sittingStatus` (`|GetArrayItem` _outactors)))
        (if (not _isplayersitting)
          (`WidgetBlueprintLibrary.SetInputMode_GameOnly` (`GameplayStatics.GetPlayerController` 0)))))
    (:`else`)))

(event `/Game/actorManagers/startTalking.endDialogue`
  (params (`isOnPC?` :type Boolean))
  (if (`/Game/widgets/dialogueWidget/dialogue.doneTalking?` (`self.widget`))
    (`Widget.RemoveFromParent` (`self.widget`))
    (bind _calling_actor (`self.Calling Actor`)
      (:`then`
        (message `/Game/actorManagers/startTalking.endDialogue` _calling_actor false))
      (:`else`))))

(fn `UserConstructionScript`)