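; Quest manager actor that tracks active quests and displays them in a quest widget.
; On BeginPlay it creates the widget, loads the "Intro" quest from a data table and starts a looping timer that refreshes all quests each second.
; UpdateQuest finds the quest by name through GetQuest and increments its stored progress by one.
; The completion check is an empty stub, and GetQuest prints an error for every non-matching entry it passes.
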(event `self.ReceiveBeginPlay`
  (bind _returnvalue (`|CreateWidget` "/Game/widgets/QuestWidget/QuestWidgetUI.QuestWidgetUI_C" (`GameplayStatics.GetPlayerController` 0)))
  (set `self.Widget` _returnvalue)
  (`UserWidget.AddToViewport` (`self.Widget`) 0)
  (`self.StartIntroEvent`)
  (`KismetSystemLibrary.K2_SetTimerDelegate` (delegate `TimedUpdate`) 1.0 true))

(event `TimedUpdate`
  (`/Game/widgets/QuestWidget/QuestWidgetUI.UpdateAllQuests` (`self.Widget`) (`self.ActiveQuests`)))

(event `StartIntroEvent`
  (bind _returnvalue (`|GetDataTableRow` (`self.dataTable`) "Intro")
    (:`then`
      (bind _output_get (set `self.currQuest` _returnvalue))
      (`KismetArrayLibrary.Array_Append` (`self.ActiveQuests`) (`|MakeArray` _output_get))
      (`/Game/widgets/QuestWidget/QuestWidgetUI.CreateQuest` (`self.Widget`) (`self.currQuest`)))
    (:`RowNotFound`
      (`KismetSystemLibrary.PrintText` "QUEST NOT FOUND"))))

(event `self.ReceiveTick`
  (params (DeltaSeconds :type "Float (single-precision)")))

(event `/Game/actorManagers/Quests/Quest_Interface.UpdateQuest`
  (params (QuestUpdate :type "/Game/actorManagers/Quests/Quest Structure"))
  (bind (_questname _currentvalue) (break `/Game/actorManagers/Quests/Quest` QuestUpdate))
  (`KismetSystemLibrary.PrintString` (`KismetStringLibrary.Conv_DoubleToString` _currentvalue) true true (struct :`R` 1.0 :`G` 0.232862 :`A` 1.0) 12.0)
  (bind (_currquest _questindex) (`self.getQuest` _questname))
  (bind _structout (setmembers `/Game/actorManagers/Quests/Quest` :`StructRef` _currquest :`CurrentValue` (+ (`.CurrentValue_5_E0F37B5042C2816B6D51B3A057987182` (break `/Game/actorManagers/Quests/Quest` _currquest)) 1.0)))
  (`KismetArrayLibrary.Array_Set` (`self.ActiveQuests`) _questindex _structout)
  (bind (_questname_2 _currentvalue_2 _desiredvalue) (break `/Game/actorManagers/Quests/Quest` _currquest))
  (if (>= _currentvalue_2 _desiredvalue)
    _))

(fn `getQuest`
  (params (quest :type String))
  (returns (currQuest :type "/Game/actorManagers/Quests/Quest Structure") (QuestIndex :type Integer))
  (for (_array_element _array_index) (`self.ActiveQuests`)
    (if (== (`.QuestName_2_C85A3B0F461CFF54C33C148B2A41309A` (break `/Game/actorManagers/Quests/Quest` _array_element)) quest)
      (return _array_element _array_index)
      (else
        (`KismetSystemLibrary.PrintString` "ERROR in GET QUEST FUNC" true true (struct :`R` 1.0 :`G` 0.092474 :`A` 1.0) 12.0)))))

(fn `UserConstructionScript`)