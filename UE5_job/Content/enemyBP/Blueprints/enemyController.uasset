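; AI controller for the closet enemy that runs BT_Enemy and teleports the enemy between approach points.
; BeginPlay finds the enemy actor and three closet teleport markers by actor tag.
; Possess starts the behavior tree and seeds the aggro and approach Blackboard keys.
; When Tick sees the ApproachingPlayer gameplay tag, it moves the enemy's XY to the marker indexed by PlayerApproach minus one, then clears the tag.
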(event `self.ReceiveBeginPlay`
  (bind _outactors (`GameplayStatics.GetAllActorsWithTag` "enemyCloset"))
  (set `self.enemyActor` (`|GetArrayItem` _outactors))
  (for _index (range 3)
    (bind _outactors_2 (`GameplayStatics.GetAllActorsWithTag` (`KismetStringLibrary.Conv_StringToName` (`KismetStringLibrary.Concat_StrStr` "closetTp" (`KismetStringLibrary.Conv_IntToString` _index)))))
    (`KismetArrayLibrary.Array_Add` (`self.tpLocations`) (`|GetArrayItem` _outactors_2))))

(event `self.ReceiveTick`
  (params (DeltaSeconds :type "Float (single-precision)"))
  (bind (_returnvalue_x _returnvalue_y) (`KismetMathLibrary.BreakVector` (`self.K2_GetActorLocation` (`|GetArrayItem` (`self.tpLocations`) (- (`self.playerApproachLoc`) 1)))))
  (if (`BlueprintGameplayTagLibrary.HasTag` (`self.gameplayContainer`) (struct :`TagName` "State.Enemy.ApproachingPlayer") true)
    (set `self.playerApproachLoc` (`BlackboardComponent.GetValueAsInt` (`self.Blackboard`) (`self.playerApproach`)))
    (`self.K2_SetActorLocation` (`self.enemyActor`) (`KismetMathLibrary.MakeVector` _returnvalue_x _returnvalue_y) false false)
    (`KismetSystemLibrary.PrintString` "Approach tag removed")
    (`BlueprintGameplayTagLibrary.RemoveGameplayTag` (`self.gameplayContainer`) (struct :`TagName` "State.Enemy.ApproachingPlayer"))))

(event `self.ReceivePossess`
  (params (PossessedPawn :type "Pawn Object Reference"))
  (`self.RunBehaviorTree` "/Game/enemyBP/Blueprints/BT_Enemy.BT_Enemy")
  (`BlackboardComponent.SetValueAsInt` (`self.Blackboard`) (`self.aggro Name`) 12)
  (`BlackboardComponent.SetValueAsInt` (`self.Blackboard`) (`self.playerApproach`) 0))

(fn `UserConstructionScript`)