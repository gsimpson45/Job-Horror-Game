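; AI controller for the window enemy, which moves in stages toward an attack at a window and can be driven back by light.
; On possess it runs BT_WindowEnemy and seeds its blackboard; BeginPlay caches tagged teleport points.
; Tick teleports the pawn to the point matching the AggroPos key.
; Interaction rolls AggroLevel against a random number and, unless attacking, may reset the enemy to the first point, clearing approach and idle tags.
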(event `self.ReceiveBeginPlay`
  (bind _aswindow_enemy (cast `/Game/enemyBP/Blueprints/windowEnemyBP/windowEnemy` (`self.K2_GetPawn` (`AIBlueprintHelperLibrary.GetAIController` self))))
  (set `self.As Window Enemy` _aswindow_enemy)
  (for _index (range 3)
    (bind _returnvalue (`KismetStringLibrary.Concat_StrStr` "windowTp" (`KismetStringLibrary.Conv_IntToString` _index)))
    (bind _outactors (`GameplayStatics.GetAllActorsWithTag` (`KismetStringLibrary.Conv_StringToName` _returnvalue)))
    (`KismetArrayLibrary.Array_Add` (`self.tpLocations`) (`|GetArrayItem` _outactors))
    (`KismetSystemLibrary.PrintString` _returnvalue)))

(event `self.ReceiveTick`
  (params (DeltaSeconds :type "Float (single-precision)"))
  (bind _output_get (set `self.index` (`BlackboardComponent.GetValueAsInt` (`self.Blackboard`) (`self.aggroPos`))))
  (switch `int` _output_get
    (:`Default`
      (`KismetSystemLibrary.PrintString` "No value received"))
    (:`0`
      (`KismetSystemLibrary.PrintString` "Go to window" false false)
      (`self.K2_SetActorLocation` (`self.As Window Enemy`) (`self.K2_GetActorLocation` (`|GetArrayItem` (`self.tpLocations`) (`self.index`))) false true :!label _label))
    (:`1`
      (`KismetSystemLibrary.PrintString` "Enemy at winoow" false false)
      (goto _label))
    (:`2`
      (`KismetSystemLibrary.PrintString` "Attack" false false)
      (goto _label))))

(event `self.ReceivePossess`
  (params (PossessedPawn :type "Pawn Object Reference"))
  (`self.RunBehaviorTree` "/Game/enemyBP/Blueprints/windowEnemyBP/BT_WindowEnemy.BT_WindowEnemy")
  (`BlackboardComponent.SetValueAsInt` (`self.Blackboard`) (`self.aggroLevel`) 12)
  (`BlackboardComponent.SetValueAsInt` (`self.Blackboard`) (`self.playerApproach`) 0)
  (`BlackboardComponent.SetValueAsObject` (`self.Blackboard`) (`self.playerObj`) "/Game/FirstPerson/Blueprints/BP_FirstPersonCharacter.BP_FirstPersonCharacter"))

(event `/Game/FirstPerson/Blueprints/BPI_flashLightInteract.interactWindowEnemy`
  (params (enemy :type "Actor Object Reference"))
  (`KismetSystemLibrary.PrintString` "HIT___________AH THE LIGHT!")
  (bind _returnval (`self.shouldRetreat`))
  (if _returnval
    (`self.K2_SetActorLocation` (`self.As Window Enemy`) (`self.K2_GetActorLocation` (`|GetArrayItem` (`self.tpLocations`))) false true)
    (`BlackboardComponent.SetValueAsInt` (`self.Blackboard`) (`self.aggroPos`) 0)
    (`BlueprintGameplayTagLibrary.RemoveGameplayTag` (`self.gameplayContainer`) (struct :`TagName` "State.Enemy.ApproachingPlayer"))
    (`BlueprintGameplayTagLibrary.RemoveGameplayTag` (`self.gameplayContainer`) (struct :`TagName` "State.Enemy.AttackIdle"))))

(fn `shouldRetreat`
  (returns (returnval :type Boolean))
  (if (and (< (`BlackboardComponent.GetValueAsInt` (`AIBlueprintHelperLibrary.GetBlackboard` null) (`self.aggroLevel`)) (`KismetMathLibrary.RandomInteger` 40)) (not (`BlueprintGameplayTagLibrary.HasTag` (`self.gameplayContainer`) (struct :`TagName` "State.Enemy.AttackPlayer"))))
    (`KismetSystemLibrary.PrintString` "Retreating")
    (return true)
    (else
      (`KismetSystemLibrary.PrintString` "Retreat failed")
      (return false))))

(fn `UserConstructionScript`)