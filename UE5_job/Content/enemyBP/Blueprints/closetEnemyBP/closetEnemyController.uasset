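; AI controller for the closet enemy, which closes on the player in teleport steps and chases them when attacking.
; On possess it runs BT_ClosetEnemy and seeds its blackboard; BeginPlay caches the tagged enemy and three closetTp markers.
; Tick polls gameplay tags: AttackPlayer triggers AIMoveTo the player.
; Otherwise, ApproachingPlayer moves the enemy to the current marker's X/Y, clears that tag and increments the blackboard step counter.
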(event `self.ReceiveBeginPlay`
  (bind _outactors (`GameplayStatics.GetAllActorsWithTag` "enemyCloset"))
  (set `self.enemyActor` (`|GetArrayItem` _outactors))
  (for _index (range 3)
    (bind _outactors_2 (`GameplayStatics.GetAllActorsWithTag` (`KismetStringLibrary.Conv_StringToName` (`KismetStringLibrary.Concat_StrStr` "closetTp" (`KismetStringLibrary.Conv_IntToString` _index)))))
    (bind _output (`|GetArrayItem` _outactors_2))
    (`KismetArrayLibrary.Array_Add` (`self.tpLocations`) _output)
    (`KismetSystemLibrary.PrintString` (`KismetSystemLibrary.GetDisplayName` _output))))

(event `self.ReceiveTick`
  (params (DeltaSeconds :type "Float (single-precision)"))
  (bind (_returnvalue_x _returnvalue_y) (`KismetMathLibrary.BreakVector` (`self.K2_GetActorLocation` (`|GetArrayItem` (`self.tpLocations`) (`self.playerApproachLoc`)))))
  (set `self.playerApproachLoc` (`BlackboardComponent.GetValueAsInt` (`self.Blackboard`) (`self.playerApproach`)))
  (if (`BlueprintGameplayTagLibrary.HasTag` (`self.gameplayContainer`) (struct :`TagName` "State.Enemy.AttackPlayer") true)
    (`|AIMoveTo` (`self.K2_GetPawn` self) (0.0 0.0 0.0) (`GameplayStatics.GetPlayerCharacter` 0))
    (elif (`BlueprintGameplayTagLibrary.HasTag` (`self.gameplayContainer`) (struct :`TagName` "State.Enemy.ApproachingPlayer") true)
      (`KismetSystemLibrary.PrintString` (`KismetStringLibrary.Conv_IntToString` (`self.playerApproachLoc`)) true true (struct :`R` 1.0 :`B` 0.169777 :`A` 1.0))
      (`self.K2_SetActorLocation` (`self.enemyActor`) (`KismetMathLibrary.MakeVector` _returnvalue_x _returnvalue_y) false false)
      (`KismetSystemLibrary.PrintString` "Approach tag removed")
      (`BlueprintGameplayTagLibrary.RemoveGameplayTag` (`self.gameplayContainer`) (struct :`TagName` "State.Enemy.ApproachingPlayer"))
      (`BlackboardComponent.SetValueAsInt` (`self.Blackboard`) (`self.playerApproach`) (+ (`self.playerApproachLoc`) 1)))))

(event `self.ReceivePossess`
  (params (PossessedPawn :type "Pawn Object Reference"))
  (`self.RunBehaviorTree` "/Game/enemyBP/Blueprints/closetEnemyBP/BT_ClosetEnemy.BT_ClosetEnemy")
  (`BlackboardComponent.SetValueAsInt` (`self.Blackboard`) (`self.aggro Name`) 22)
  (`BlackboardComponent.SetValueAsInt` (`self.Blackboard`) (`self.playerApproach`) 0)
  (`BlackboardComponent.SetValueAsObject` (`self.Blackboard`) (`self.playerObj`) "/Game/FirstPerson/Blueprints/BP_FirstPersonCharacter.BP_FirstPersonCharacter"))

(fn `UserConstructionScript`)