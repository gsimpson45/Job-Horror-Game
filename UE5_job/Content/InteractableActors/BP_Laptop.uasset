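; BP_Laptop is an interactable laptop that shows a live screen on its mesh and switches the player to it on use.
; Construction creates a dynamic material on the mesh's second slot, and Tick feeds the Screen's render target into it.
; Starting interaction sets UI-only input and blends the view to the first actor tagged NyraLaptop.
; Ending interaction only calls the parent, as the code restoring game input and player view is unconnected.
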(event `self.ReceiveBeginPlay`)

(event `self.ReceiveTick`
  (params (DeltaSeconds :type "Float (single-precision)"))
  (`MaterialInstanceDynamic.SetTextureParameterValue` (`self.dynamicMaterial`) "screenImage" (`WidgetComponent.GetRenderTarget` (`self.screen`))))

(event `self.Start interaction`
  (`parent.Start interaction`)
  (`WidgetBlueprintLibrary.SetInputMode_UIOnlyEx` (`GameplayStatics.GetPlayerController` 0) null)
  (bind _outactors (`GameplayStatics.GetAllActorsWithTag` "NyraLaptop"))
  (`PlayerController.SetViewTargetWithBlend` (`GameplayStatics.GetPlayerController` 0) (`|GetArrayItem` _outactors) 1.0 "VTBlend_Linear" 0.0 true))

(event `self.End interaction`
  (`parent.End interaction`))

(event `/Game/FirstPerson/Blueprints/BPI_LookAt.MCLookAt`
  (`parent.MCLookAt`))

(event `/Game/FirstPerson/Blueprints/BPI_LookAt.MCLookAway`
  (`parent.MCLookAway`))

(fn `UserConstructionScript`
  (bind _returnvalue (`PrimitiveComponent.CreateDynamicMaterialInstance` (`self.rr`) 1 "/Game/widgets/MI_InteractiveScreen_Inst.MI_InteractiveScreen_Inst" "None"))
  (set `self.dynamicMaterial` _returnvalue))