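; BP_Bed is an interactable bed actor that shows a "Sleeptime!" prompt and plays a go-to-sleep sequence when used.
; On interaction start it sends the player toward a stand location, stops movement after a short fixed delay, then creates and plays the GoToSleepAnim level sequence.
; It extends a parent interactable's events, with end-interaction and look-at handlers only forwarding to the parent.
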(event `self.Start interactiom`
  (`parent.Start interactiom`)
  (`AIBlueprintHelperLibrary.SimpleMoveToLocation` (`GameplayStatics.GetPlayerController` 0) (`SceneComponent.K2_GetComponentLocation` (`self.standLocation`)))
  (`KismetSystemLibrary.Delay` 0.5)
  (`Controller.StopMovement` (`GameplayStatics.GetPlayerController` 0))
  (bind _outactor (`LevelSequencePlayer.CreateLevelSequencePlayer` "/Game/CharacterAnimations/GoToSleepAnim.GoToSleepAnim" (`self.Settings`)))
  (bind _output_get (set `self.Sequence Player` (`LevelSequenceActor.SequencePlayer` _outactor)))
  (`MovieSceneSequencePlayer.Play` _output_get))

(event `self.End interaction`
  (`parent.End interaction`))

(event `self.promptInteraction`
  (set `self.interactPopupText` "Sleeptime!")
  (`parent.promptInteraction`))

(event `/Game/FirstPerson/Blueprints/BPI_LookAt.MCLookAt`
  (`parent.MCLookAt`))

(event `/Game/FirstPerson/Blueprints/BPI_LookAt.MCLookAway`
  (`parent.MCLookAway`))

(fn `UserConstructionScript`)