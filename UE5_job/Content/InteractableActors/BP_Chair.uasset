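; BP_Chair is an interactable chair the player can either sit on or hide at.
; Interacting blends to a tagged screen camera, adds the SittingCamControls widget in UI-only input and sets a Sitting tag on the player controller.
; Releasing Q toggles hiding during interaction when not seated, blending to a hide camera with a level sequence, or back to the character.
; Gameplay tags on the controller block sit logic while hiding.
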(event `self.Start interactiom`
  (`parent.Start interactiom`)
  (if (not (`BlueprintGameplayTagLibrary.HasTag` (`/Game/FirstPerson/Blueprints/BP_FirstPersonPlayerController.gameplayContainerPL` (`self.As BP First Person Player Controller`)) (struct :`TagName` "State.Player.Interact.Hiding")))
    (`KismetSystemLibrary.PrintString` "casting parentinteraction called")
    (bind _ascharacter (cast `Character` (`self.playerActor`)))
    (set `self.As Character` _ascharacter)
    (bind _outactors (`GameplayStatics.GetAllActorsWithTag` "screenCameraTag"))
    (bind _returnvalue (`|CreateWidget` "/Game/widgets/sittingCamControls.sittingCamControls_C" (`GameplayStatics.GetPlayerController` 0)))
    (bind _output_get (set `self.widget` _returnvalue))
    (`UserWidget.AddToViewport` _output_get 0)
    (`PlayerController.SetViewTargetWithBlend` (`GameplayStatics.GetPlayerController` 0) (`|GetArrayItem` _outactors) 1.0 "VTBlend_Linear" 0.0 false)
    (`WidgetBlueprintLibrary.SetInputMode_UIOnlyEx` (`GameplayStatics.GetPlayerController` 0) null)
    (set `self.isSitting` true)
    (`KismetSystemLibrary.PrintString` "IN UI MODE")
    (`BlueprintGameplayTagLibrary.AddGameplayTag` (`/Game/FirstPerson/Blueprints/BP_FirstPersonPlayerController.gameplayContainerPL` (`self.As BP First Person Player Controller`)) (struct :`TagName` "State.Player.Interact.Sitting"))))

(event `self.End interaction`
  (`parent.End interaction`)
  (if (not (`BlueprintGameplayTagLibrary.HasTag` (`/Game/FirstPerson/Blueprints/BP_FirstPersonPlayerController.gameplayContainerPL` (`self.As BP First Person Player Controller`)) (struct :`TagName` "State.Player.Interact.Hiding")))
    (set `self.cameraToFind` null)
    (set `self.isSitting` false)
    (`Widget.RemoveFromParent` (`self.Widget`))))

(event `Key|Q`
  (params (Key :type "Key Structure"))
  (bind _returnvalue (`GameplayStatics.GetPlayerController` 0))
  (:`Released`
    (`KismetSystemLibrary.PrintString` "Hide")
    (bind _asbp_first_person_player_controller (cast `/Game/FirstPerson/Blueprints/BP_FirstPersonPlayerController` (`GameplayStatics.GetPlayerController` 0)))
    (set `self.As BP First Person Player Controller` _asbp_first_person_player_controller)
    (bind _outactor (`LevelSequencePlayer.CreateLevelSequencePlayer` "/Game/cameraAnim/hideAnim.hideAnim" (`self.Settings`)))
    (set `self.sitCamera` _outactor)
    (if (`BlueprintGameplayTagLibrary.HasTag` (`/Game/FirstPerson/Blueprints/BP_FirstPersonPlayerController.gameplayContainerPL` (`self.As BP First Person Player Controller`)) (struct :`TagName` "State.Player.Interact.Hiding"))
      (`BlueprintGameplayTagLibrary.RemoveGameplayTag` (`/Game/FirstPerson/Blueprints/BP_FirstPersonPlayerController.gameplayContainerPL` (`self.As BP First Person Player Controller`)) (struct :`TagName` "State.Player.Interact.Hiding"))
      (`self.SetActorHiddenInGame` (`GameplayStatics.GetPlayerPawn` 0) false)
      (`self.K2_SetActorRelativeRotation` (`self.As BP First Person Player Controller`) (struct :`Yaw` -180.0) false true)
      (`KismetSystemLibrary.PrintString` "done hiding")
      (bind _asbp_first_person_character (cast `/Game/FirstPerson/Blueprints/BP_FirstPersonCharacter` (`Controller.K2_GetPawn` _returnvalue)))
      (`PlayerController.SetViewTargetWithBlend` _returnvalue _asbp_first_person_character 1.0 "VTBlend_Linear" 0.6 false)
      (`KismetSystemLibrary.PrintString` "Leave hide anim")
      (bind _outactors (`GameplayStatics.GetAllActorsWithTag` "hideCameraAnim" :!label _label))
      (elif (and (`self.isInteraction`) (not (`self.isSitting`)))
        (`BlueprintGameplayTagLibrary.AddGameplayTag` (`/Game/FirstPerson/Blueprints/BP_FirstPersonPlayerController.gameplayContainerPL` (`self.As BP First Person Player Controller`)) (struct :`TagName` "State.Player.Interact.Hiding"))
        (bind _outactors_2 (`GameplayStatics.GetAllActorsWithTag` "hideCameraAnim"))
        (`PlayerController.SetViewTargetWithBlend` (`GameplayStatics.GetPlayerController` 0) (`|GetArrayItem` _outactors_2) 0.1 "VTBlend_Linear" 0.0 false)
        (`MovieSceneSequencePlayer.Play` (`LevelSequenceActor.SequencePlayer` (`self.sitCamera`)))
        (`KismetSystemLibrary.PrintString` "hide anim")
        (goto _label)
        (else
          (`KismetSystemLibrary.PrintString` "cannot hide when sitting"))))))

(event `self.ReceiveBeginPlay`
  (bind _asbp_first_person_player_controller (cast `/Game/FirstPerson/Blueprints/BP_FirstPersonPlayerController` (`GameplayStatics.GetPlayerController` 0)))
  (set `self.As BP First Person Player Controller` _asbp_first_person_player_controller))

(fn `sittingStatus`
  (returns (isPlayerSitting :type Boolean))
  (return (`self.isSitting`)))

(fn `UserConstructionScript`
  (`parent.UserConstructionScript`))