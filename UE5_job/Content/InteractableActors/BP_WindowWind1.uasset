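; BP_WindowWind1 is an interactable window actor with a hold-E progress prompt.
; BeginPlay creates a collapsed WindowInteraction widget, shown when a player character overlaps and hidden on any overlap end, as that player check is unused.
; Tick raises the widget's percent while E is held in range and otherwise lowers it at half rate, stepping by frame delta minus the delta saved on E release.
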(event `self.ReceiveTick`
  (params (DeltaSeconds :type "Float (single-precision)"))
  (bind _widget (`self.widget`))
  (bind _widget_2 (`self.widget`))
  (set `self.Delta Seconds` DeltaSeconds)
  (if (and (`self.isEPressed`) (`self.isInteracting`))
    (bind _output_get (set `self.timer` (- (`self.Delta Seconds`) (`self.startTime`))))
    (set `/Game/widgets/objectInteraction/windowInteraction.percent` (+ (`/Game/widgets/objectInteraction/windowInteraction.percent` _widget_2) _output_get) _widget_2)
    (`KismetSystemLibrary.PrintString` "clicking")
    (else
      (bind _output_get_2 (set `self.timer` (- (`self.Delta Seconds`) (`self.startTime`))))
      (set `/Game/widgets/objectInteraction/windowInteraction.percent` (- (`/Game/widgets/objectInteraction/windowInteraction.percent` _widget) (/ _output_get_2 2.0)) _widget))))

(event `Key|E` :consume false
  (params (Key :type "Key Structure"))
  (:`Pressed`
    (set `self.isEPressed` true)
    (if (`self.isInteracting`)
      (`KismetSystemLibrary.PrintString` "e pressed in window")))
  (:`Released`
    (set `self.isEPressed` false)
    (set `self.startTime` (`self.Delta Seconds`))))

(event `self.ReceiveBeginPlay`
  (bind _returnvalue (`|CreateWidget` "/Game/widgets/objectInteraction/windowInteraction.windowInteraction_C" (`GameplayStatics.GetPlayerController` 0)))
  (bind _output_get (set `self.widget` _returnvalue))
  (`UserWidget.AddToViewport` _output_get 0)
  (set `Widget.Visibility` "Collapsed" (`self.widget`)))

(event `self.ReceiveActorBeginOverlap`
  (params (OtherActor :type "Actor Object Reference"))
  (set `self.currActor` OtherActor)
  (bind _isplayer (message `/Game/FirstPerson/Blueprints/BPI_character.isPlayerChar` OtherActor))
  (if _isplayer
    (set `self.isInteracting` true)
    (set `Widget.Visibility` "Visible" (`self.widget`))
    (`KismetSystemLibrary.PrintString` "overlapping")))

(event `self.ReceiveActorEndOverlap`
  (params (OtherActor :type "Actor Object Reference"))
  (message `/Game/FirstPerson/Blueprints/BPI_character.isPlayerChar` OtherActor)
  (if true
    (set `self.isInteracting` false)
    (set `Widget.Visibility` "Collapsed" (`self.widget`))))

(fn `UserConstructionScript`)